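; BP_Topic_Unlocker is a placeable actor that unlocks dialogue topics for nearby actors in the topic dialogue system.
; When TriggerByOverlap is set, the construction script adds a sphere of UnlockRadius and binds its begin-overlap event.
; SendUnlockTopicBroadcast sphere-queries WorldDynamic and Pawn actors within that radius and unlocks every TopicsToUnlock entry on each TopicManagerComponent found.
; Overlaps trigger this broadcast without filtering the entering actor, and debug prints report progress.
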(event `Handle Overlap Sphere`
  (params (OverlappedComponent :type "PrimitiveComponent Object Reference") (OtherActor :type "Actor Object Reference") (OtherComp :type "PrimitiveComponent Object Reference") (OtherBodyIndex :type Integer) (bFromSweep :type Boolean) (SweepResult :type "HitResult Structure (by ref)"))
  (`self.Send Unlock Topic Broadcast`))

(fn `Send Unlock Topic Broadcast`
  (`KismetSystemLibrary.PrintString` (`KismetStringLibrary.Concat_StrStr` "Unlocking Topcis starting at: " (`KismetStringLibrary.Conv_NameToString` (`|GetArrayItem` (`self.Topics To Unlock`)))))
  (bind _outactors (`KismetSystemLibrary.SphereOverlapActors` (`self.K2_GetActorLocation`) (`self.Unlock Radius`) (`|MakeArray` "ObjectTypeQuery2" "ObjectTypeQuery3" :!type "EObjectTypeQuery Enum")))
  (for _array_element _outactors
    (bind _returnvalue (`self.GetComponentByClass` _array_element "/Script/TopicDialogueSystem.TopicManagerComponent"))
    (`/Engine/EditorBlueprintResources/StandardMacros.IsValid` _returnvalue
      (:`Is Valid`
        (for _array_element_2 (`self.Topics To Unlock`)
          (`TopicManagerComponent.UnlockDialogueTopic` _returnvalue _array_element_2)
          (`KismetSystemLibrary.PrintString` "sucess unlock!"))))))

(fn `UserConstructionScript`
  (if (`self.Trigger By Overlap`)
    (bind _returnvalue (`AddComponent|NODE_AddSphereComponent-0`))
    (`SphereComponent.SetSphereRadius` _returnvalue (`self.Unlock Radius`) true)
    (add `PrimitiveComponent.OnComponentBeginOverlap` _returnvalue (`|CreateDelegate` :!event `Handle Overlap Sphere`))))